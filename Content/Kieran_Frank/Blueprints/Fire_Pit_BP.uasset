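; Fire pit trigger that sets the player character on fire when it enters the box, depending on its material.
; Overlap reads the first Player_Character's MaterialString: Wood and Ice both ignite with sound and a damage binding, but only Wood unhides the point light.
; The generated damage handler extinguishes the character, hides the light and unbinds damage events unless its Material is one of two enum values.
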(event `self.Box.OnComponentBeginOverlap`
  (params (OverlappedComponent :type "PrimitiveComponent Object Reference") (OtherActor :type "Actor Object Reference") (OtherComp :type "PrimitiveComponent Object Reference") (OtherBodyIndex :type Integer) (bFromSweep :type Boolean) (SweepResult :type "HitResult Structure (by ref)"))
  (bind _asplayer_character (cast `/Game/Player_Character_Liam/Player_Character` OtherActor))
  (bind _outactors (`GameplayStatics.GetAllActorsOfClass` "/Game/Player_Character_Liam/Player_Character.Player_Character_C"))
  (bind _material_string (`/Game/Player_Character_Liam/Player_Character.Material_String` (`|GetArrayItem` _outactors)))
  (if (`KismetStringLibrary.EqualEqual_StrStr` _material_string "Wood")
    (`SceneComponent.SetHiddenInGame` (`/Game/Player_Character_Liam/Player_Character.PointLight` _asplayer_character) false false)
    (set `/Game/Player_Character_Liam/Player_Character.On Fire?` true _asplayer_character)
    (add `self.OnTakeAnyDamage` _asplayer_character (`|CreateDelegate` :!event `Fire_Pit_BP_AutoGenFunc`) :!label _label)
    (`GameplayStatics.PlaySound2D` "/Game/Sarah_Roddam/Audio/LevelSFX/Fire_Torch_Cue.Fire_Torch_Cue" 1.0 1.0 0.0 null null)
    (`KismetSystemLibrary.PrintString` "on fire")
    (elif (`KismetStringLibrary.EqualEqual_StrStr` _material_string "Ice")
      (set `/Game/Player_Character_Liam/Player_Character.On Fire?` true _asplayer_character)
      (goto _label))))

(fn `Fire_Pit_BP_AutoGenFunc`
  (params (DamagedActor :type "Actor Object Reference") (Damage :type "Float (double-precision)") (DamageType :type "DamageType Object Reference") (InstigatedBy :type "Controller Object Reference") (DamageCauser :type "Actor Object Reference"))
  (bind _asplayer_character (cast `/Game/Player_Character_Liam/Player_Character` DamagedActor))
  (bind _material (`/Game/Player_Character_Liam/Player_Character.Material` _asplayer_character))
  (if (not (or (`|EnumEquality` _material "NewEnumerator2") (`|EnumEquality` _material "NewEnumerator1")))
    (set `/Game/Player_Character_Liam/Player_Character.On Fire?` false _asplayer_character)
    (`SceneComponent.SetVisibility` (`/Game/Player_Character_Liam/Player_Character.PointLight` _asplayer_character) false false)
    (clear `self.OnTakeAnyDamage` _asplayer_character)))

(fn `UserConstructionScript`)